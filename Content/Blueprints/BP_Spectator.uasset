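; Multiplayer spectator that views the game through the first BP_BikePlayer and measures the loudness of captured audio.
; On BeginPlay it sets that view target and adds an audio capture component, except on Android instances without authority.
; Non-authority instances sum the audio envelope values over roughly one-second windows, then pass each total through SetSumOnServer to store as LastKnownSum.
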(event Custom|OnAudioEnvelopeValue_Event_0
  (params (EnvelopeValue :type Float%20%28single-precision%29))
  (Networking|SwitchHasAuthority
    (:Remote
      (Variables|Default|SetEnvelopeSUm (+ (Variables|Default|GetEnvelopeSUm) EnvelopeValue)))))

(event Custom|SetSumOnServer
  (params (EnvelopeSUm :type Float%20%28single-precision%29))
  (Variables|Default|SetLastKnownSum EnvelopeSUm))

(event EventBeginPlay
  (bind _outactors (Actor|GetAllActorsOfClass "/Game/Blueprints/Player/BP_BikePlayer.BP_BikePlayer_C"))
  (Game|Player|SetViewTargetwithBlend (Game|GetPlayerController 0) (Utilities|Array|Get(acopy) _outactors) 0.0 "VTBlend_Linear" 0.0 false)
  (if (not (and (Utilities|Enum|Equal(Enum) (Game|GetPlatformName) "Android") (not (Ability|HasAuthority))))
    (bind _returnvalue (AddComponent|AddAudioCaptureComponent false))
    (bind _output_get (Variables|Default|SetRuntimeAudioCapture _returnvalue))
    (Components|Activation|Activate _output_get false)
    (EventDispatchers|AssignOnAudioEnvelopeValue _output_get (delegate Custom|OnAudioEnvelopeValue_Event_0))))

(event EventTick
  (params (DeltaSeconds :type Float%20%28single-precision%29))
  (Networking|SwitchHasAuthority
    (:Remote
      (bind _output_get (Variables|Default|SetTimeElapsed (+ DeltaSeconds (Variables|Default|GetTimeElapsed))))
      (if (> _output_get 1.0)
        (Variables|Default|SetLastKnownSum (Variables|Default|GetEnvelopeSUm))
        (Variables|Default|SetTimeElapsed 0.0)
        (Variables|Default|SetEnvelopeSUm 0.0)
        (CallFunction|SetSumonServer (Variables|Default|GetLastKnownSum))))))

(fn ConstructionScript)