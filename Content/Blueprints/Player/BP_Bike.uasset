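; Self-driving bike vehicle that chases a Target actor along navmesh paths, with its Dog mesh tinted a random color.
; Each tick it re-queries the path, holds full throttle and steers by the dot product of next-segment direction and its right vector.
; Debug cylinders mark upcoming path points in the bike's color.
; Navmesh clamping is never called; look-ahead and alternative steering logic are dead code.
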(event EventBeginPlay
  (bind _dog (Variables|Default|GetDog))
  (bind _output_get (Variables|Default|SetPathColor (Utilities|Struct|MakeLinearColor (Math|Random|RandomFloat) (Math|Random|RandomFloat) (Math|Random|RandomFloat) 1.0)))
  (bind _returnvalue (Rendering|Material|CreateDynamicMaterialInstance _dog 1 "/Game/Art/Materials/M_DogMaterial.M_DogMaterial" "None" :!class /Script/Engine.PrimitiveComponent))
  (Rendering|Material|SetVectorParameterValue _returnvalue "Base color" _output_get :!class /Script/Engine.MaterialInstanceDynamic)
  (bind _returnvalue_2 (Rendering|Material|CreateDynamicMaterialInstance _dog 2 "/Game/Art/Materials/M_DogMaterial.M_DogMaterial" "None" :!class /Script/Engine.PrimitiveComponent))
  (Rendering|Material|SetVectorParameterValue _returnvalue_2 "Base color" _output_get :!class /Script/Engine.MaterialInstanceDynamic))

(event EventTick
  (params (DeltaSeconds :type Float%20%28single-precision%29))
  (CallFunction|FindPathPoints (Transformation|GetActorLocation))
  (CallFunction|CalculatePathPointForwardVector)
  (Class|WheeledVehicleMovementComponent|SetThrottleInput (Variables|Default|GetVehicleMovement) 1.0)
  (Utilities|Array|SetArrayElem (Variables|Default|GetPathToEnd) 0 (Transformation|GetActorLocation))
  (CallFunction|DrawPathDebug)
  (if true
    (CallFunction|RotatetoMatchNextPoint)
    (else
      (Class|WheeledVehicleMovementComponent|SetSteeringInput (Variables|Default|GetVehicleMovement) (Math|Vector|DotProduct (* (Transformation|GetActorRightVector) 1.0) (Variables|Default|GetForwardVectorBetweenPoints)))
      (Development|PrintString "Hello"))))

(fn ConstructionScript)

(fn PlaySoundatActorLocation
  (params (Sound :type Sound%20Base%20Object%20Reference))
  (Audio|PlaySoundatLocation Sound (Transformation|GetActorLocation) "0, 0, 0" 1.0 1.0 0.0 0 0 0))

(fn FindPathPoints
  (params (PathStart :type Vector%20%28by%20ref%29))
  (bind _target (Variables|Default|GetTarget)
    (:then
      (bind _returnvalue (Class|NavigationSystemV1|FindPathtoActorSynchronously PathStart _target 5e+01 0 0))
      (if (> (Utilities|Array|Length (Variables|/Script/NavigationSystem.NavigationPath|GetPathPoints _returnvalue)) 1)
        (Variables|Default|SetPathToEnd (Variables|/Script/NavigationSystem.NavigationPath|GetPathPoints _returnvalue))))
    (:else)))

(fn DrawPathDebug
  (bind _pathtoend (Variables|Default|GetPathToEnd))
  (for _index (range 0 5)
    (if (Utilities|Array|IsValidIndex _pathtoend _index)
      (Class|KismetSystemLibrary|DrawDebugCylinder (Utilities|Array|Get(acopy) _pathtoend _index) (+ (Utilities|Array|Get(acopy) _pathtoend _index) "0, 0,100.000000") 1e+02 12 (Variables|Default|GetPathColor) 0.0 3.0))))

(fn RotatetoMatchNextPoint
  (bind _pathtoend (Variables|Default|GetPathToEnd))
  (Class|WheeledVehicleMovementComponent|SetSteeringInput (Variables|Default|GetVehicleMovement) (Math|Vector|DotProduct (Math|Vector|Normalize (- (Utilities|Array|Get(acopy) _pathtoend 1) (Utilities|Array|Get(acopy) _pathtoend))) (Transformation|GetActorRightVector))))

(fn FindValidMovetoPoint
  (params (Scale :type Float%20%28single-precision%29)))

(fn CalculatePathPointForwardVector
  (bind _pathtoend (Variables|Default|GetPathToEnd))
  (if (Utilities|Array|IsValidIndex _pathtoend 1)
    (Variables|Default|SetForwardVectorBetweenPoints (Math|Vector|Normalize (- (Utilities|Array|Get(acopy) _pathtoend 1) (Utilities|Array|Get(acopy) _pathtoend))))))

(fn KeepActoronNavMesh
  (bind _returnvalue (Transformation|GetActorLocation))
  (bind (_projectedlocation _returnvalue_2) (AI|Navigation|ProjectPointtoNavigation _returnvalue 0 0 "0, 0, 0"))
  (if _returnvalue_2
    (Variables|Default|SetLastValidLocation _projectedlocation)
    (else
      (Transformation|SetActorLocation (Variables|Default|GetLastValidLocation) false false))))