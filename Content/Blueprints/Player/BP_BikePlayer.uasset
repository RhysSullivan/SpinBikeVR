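; VR player bike pawn that spawns motion-controller hands, forwarding grab, use and pause input to them and snap-turning the VR origin.
; Handlebar yaw drives vehicle steering and the front fork, while throttle comes from the first BikePath actor's LastKnownSum.
; Forward speed spins the wheels and scales audio volume, and a looping timer plays random dog sounds.
; Keys C and J host a Lvl_Island listen session and test session search.
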(event Custom|DoDogSound
  (bind _dog (Variables|Default|GetDog))
  (bind _returnvalue (Transformation|GetWorldTransform _dog))
  (Utilities|FlowControl|Delay (Math|Random|RandomFloatinRange 5.0 7.0))
  (Audio|SpawnSoundatLocation (Utilities|Array|Get(acopy) (Variables|Default|GetSoundArray) (Math|Random|RandomIntegerinRange 0 2)) (.location _returnvalue) (.rotation _returnvalue) 1.0 1.0 0.0 "/Game/Sound/BarkAttinuation.BarkAttinuation" 0)
  (CallFunction|DoDogSound))

(event EventBeginPlay
  (Utilities|FlowControl|Sequence
    (:then_0
      (Class|HeadMountedDisplayFunctionLibrary|ResetOrientationandPosition 0.0 "OrientationAndPosition")
      (Class|HeadMountedDisplayFunctionLibrary|SetTrackingOrigin "Eye"))
    (:then_1
      (Utilities|FlowControl|Sequence
        (:then_0
          (bind _returnvalue (Game|SpawnActorfromClass "/Game/Blueprints/Player/BP_LeftHand.BP_LeftHand_C" (Math|Transform|MakeTransform "0, 0, 0" "0, 0, 0" "1,1,1") "Undefined" 0 0))
          (bind _output_get (Variables|Default|SetBP%20Left%20Hand _returnvalue))
          (Transformation|AttachComponentToComponent _output_get (Variables|Default|GetMotionControllerLeft) "None" "SnapToTarget" "SnapToTarget" "KeepWorld" false)
          (Variables|/Game/Blueprints/Player/BP_Hand.BP_Hand_C|SetMotionControllerComponent (Variables|Default|GetBP%20Left%20Hand) (Variables|Default|GetMotionControllerLeft)))
        (:then_1
          (bind _returnvalue_2 (Game|SpawnActorfromClass "/Game/Blueprints/Player/BP_RightHand.BP_RightHand_C" (Math|Transform|MakeTransform "0, 0, 0" "0, 0, 0" "1,1,1") "Undefined" 0 0))
          (bind _output_get_2 (Variables|Default|SetBP%20Right%20Hand _returnvalue_2))
          (Transformation|AttachComponentToComponent _output_get_2 (Variables|Default|GetMotionControllerRight) "None" "SnapToTarget" "SnapToTarget" "KeepWorld" false)
          (Variables|/Game/Blueprints/Player/BP_Hand.BP_Hand_C|SetMotionControllerComponent (Variables|Default|GetBP%20Right%20Hand) (Variables|Default|GetMotionControllerRight)))))
    (:then_3
      (CallFunction|DoDogSound))))

(event EventTick
  (params (DeltaSeconds :type Float%20%28single-precision%29))
  (bind _vehiclemovement (Variables|Default|GetVehicleMovement))
  (bind _returnvalue (Class|WheeledVehicleMovementComponent|GetForwardSpeed _vehiclemovement))
  (bind _asbp_handlebars (Utilities|Casting|CastToBP_Handlebars (Variables|/Script/Engine.ChildActorComponent|GetChildActor (Variables|Default|GetBP_Handlebars))))
  (Class|WheeledVehicleMovementComponent|SetSteeringInput (Variables|Default|GetVehicleMovement) (/ (.yaw (Variables|/Script/Engine.SceneComponent|GetRelativeRotation (Variables|/Game/Blueprints/Player/BP_Handlebars.BP_Handlebars_C|GetStaticMesh _asbp_handlebars))) (Variables|/Game/Blueprints/Player/BP_Handlebars.BP_Handlebars_C|GetMaxSteeringWheelRotation _asbp_handlebars)))
  (bind _asbp_handlebars_2 (Utilities|Casting|CastToBP_Handlebars (Variables|/Script/Engine.ChildActorComponent|GetChildActor (Variables|Default|GetBP_Handlebars))))
  (Transformation|SetRelativeRotation (Variables|Default|GetFrameFrontWheelConnector) (Math|Rotator|MakeRotator 0.0 0.0 (.yaw (Variables|/Script/Engine.SceneComponent|GetRelativeRotation (Variables|/Game/Blueprints/Player/BP_Handlebars.BP_Handlebars_C|GetStaticMesh _asbp_handlebars_2)))) false false)
  (Transformation|AddLocalRotation (Variables|Default|GetWheelFront) (Math|Rotator|MakeRotator (* _returnvalue (Variables|Default|GetRotationMultiplier)) 0.0 0.0) false false)
  (Audio|Components|Audio|SetVolumeMultiplier (Variables|Default|GetAudio) (/ _returnvalue 4.5e+02) :!class /Script/Engine.AudioComponent))

(event EventDestroyed
  (Actor|DestroyActor (Variables|Default|GetBP%20Left%20Hand)))

(event Input|ActionEvents|InputActionTurnLeft
  (params (Key :type Key%20Structure :default "None"))
  (:Pressed
    (Transformation|AddWorldRotation (Variables|Default|GetVROrigin) (Math|Rotator|MakeRotator 0.0 0.0 (* (Variables|Default|GetRotationRate) -1.0)) false false)))

(event Input|ActionEvents|InputActionGrabRight
  (params (Key :type Key%20Structure :default "None"))
  (bind _bp_right_hand (Variables|Default|GetBP%20Right%20Hand))
  (:Pressed
    (Default|SendGrab _bp_right_hand))
  (:Released
    (Default|SendRelease _bp_right_hand)))

(event Input|ActionEvents|InputActionGrabLeft
  (params (Key :type Key%20Structure :default "None"))
  (bind _bp_left_hand (Variables|Default|GetBP%20Left%20Hand))
  (:Pressed
    (Default|SendGrab _bp_left_hand))
  (:Released
    (Default|SendRelease _bp_left_hand)))

(event Input|ActionEvents|InputActionUseRight
  (params (Key :type Key%20Structure :default "None"))
  (bind _bp_right_hand (Variables|Default|GetBP%20Right%20Hand))
  (bind _widgetinteraction (Variables|/Game/Blueprints/Player/BP_RightHand.BP_RightHand_C|GetWidgetInteraction _bp_right_hand))
  (:Pressed
    (Class|WidgetInteractionComponent|PressPointerKey _widgetinteraction "LeftMouseButton")
    (Utilities|FlowControl|Delay 0.2)
    (Class|WidgetInteractionComponent|ReleasePointerKey _widgetinteraction "LeftMouseButton")
    (Default|Activate (Variables|Default|GetBP%20Right%20Hand))))

(event Input|ActionEvents|InputActionPause
  (params (Key :type Key%20Structure :default "None"))
  (:Pressed
    (Default|Pause (Variables|Default|GetBP%20Left%20Hand))))

(event Input|ActionEvents|InputActionTurnRight
  (params (Key :type Key%20Structure :default "None"))
  (:Pressed
    (Transformation|AddWorldRotation (Variables|Default|GetVROrigin) (Math|Rotator|MakeRotator 0.0 0.0 (Variables|Default|GetRotationRate)) false false)))

(event Input|ActionEvents|InputActionToggleLaserPointer
  (params (Key :type Key%20Structure :default "None"))
  (bind _bp_right_hand (Variables|Default|GetBP%20Right%20Hand))
  (bind _widgetinteraction (Variables|/Game/Blueprints/Player/BP_RightHand.BP_RightHand_C|GetWidgetInteraction _bp_right_hand))
  (:Pressed
    (Variables|/Script/UMG.WidgetInteractionComponent|SetbShowDebug _widgetinteraction (not (Variables|/Script/UMG.WidgetInteractionComponent|GetbShowDebug _widgetinteraction)))))

(event Input|AxisEvents|InputAxisMoveLeft
  (params (AxisValue :type Float%20%28single-precision%29)))

(event Input|AxisEvents|InputAxisMoveForward
  (params (AxisValue :type Float%20%28single-precision%29))
  (bind _outactors (Actor|GetAllActorsOfClass "/Script/SpinBikeVR.BikePath"))
  ;[1 1 1] Throttle input
  (if (Utilities|Array|IsValidIndex _outactors)
    (Class|WheeledVehicleMovementComponent|SetThrottleInput (Variables|Default|GetVehicleMovement) (Variables|/Script/SpinBikeVR.BikePath|GetLastKnownSum (Utilities|Array|Get(acopy) _outactors)))))

(event Input|KeyboardEvents|C
  (params (Key :type Key%20Structure :default "None"))
  (:Pressed
    (|Session (Game|GetPlayerController 0) 2 false
      (:OnSuccess
        (Game|OpenLevel(byName) "Lvl_Island" true "?listen")))))

(event Input|KeyboardEvents|J
  (params (Key :type Key%20Structure :default "None"))
  (:Pressed
    (bind _results (|FindSessions (Game|GetPlayerController 0) 0 false)
      (:then
        (for _array_element _results
          (Development|PrintString "Hello"))))))

(fn ConstructionScript)

(fn PlaySoundatActorLocation
  (params (Sound :type Sound%20Base%20Object%20Reference))
  (Audio|PlaySoundatLocation Sound (Transformation|GetActorLocation) "0, 0, 0" 1.0 1.0 0.0 0 0 0))