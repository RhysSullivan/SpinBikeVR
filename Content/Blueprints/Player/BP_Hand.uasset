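; BP_Hand is a motion-controller hand actor that grabs and releases objects it touches.
; SendGrab sends a grab message, with hand side and controller, to actors overlapping its sphere, storing the first successful result as GrabbedActor.
; SendRelease messages that actor and clears the reference when release succeeds.
; Its own Grab and Release functions only return false, and collision toggles in SetGrabbedActor are unconnected.
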(event Custom|Send%20Grab
  (bind _array_element (Utilities|Array|ForEachLoopwithBreak (Collision|GetOverlappingActors (Variables|Default|GetSphere) 0 :!class /Script/Engine.PrimitiveComponent))
    (:LoopBody
      (bind (_success _grabbedactor) (Class|BPWorldInteractionInterface|Grab(Message) _array_element (Variables|/Script/HeadMountedDisplay.MotionControllerComponent|GetHand (Variables|Default|GetMotionControllerComponent)) self (Variables|Default|GetMotionControllerComponent) "None"))
      (if _success
        (Variables|Default|SetGrabbedActor _grabbedactor)
        (CallFunction|Break)))))

(event Custom|Send%20Release
  (bind _grabbedactor (Variables|Default|GetGrabbedActor)
    (:then
      (bind _success (Class|BPWorldInteractionInterface|Release(Message) _grabbedactor))
      (if _success
        (Variables|Default|SetGrabbedActor 0)))
    (:else)))

(event Custom|Break
  (Utilities|Array|ForEachLoopwithBreak (Collision|GetOverlappingActors (Variables|Default|GetSphere) 0 :!class /Script/Engine.PrimitiveComponent)) ; enters at Break
)

(fn ConstructionScript
  (|CallParentFunction))

(fn SetGrabbedActor
  (params (InputPin :type Actor%20Object%20Reference))
  (Utilities|IsValid InputPin
    (:Is%20Valid
      (Variables|Default|SetGrabbedActor InputPin))
    (:Is%20Not%20Valid
      (Variables|Default|SetGrabbedActor 0))))

(fn Grab
  (params (WhichHand :type EControllerHand%20Enum :default "Left") (GrabbingActor :type Actor%20Object%20Reference) (MotionControllerComponent :type Scene%20Component%20Object%20Reference) (Socket%20To%20Attach%20To :type Name :default "None"))
  (return false 0))

(fn Release
  (return false))