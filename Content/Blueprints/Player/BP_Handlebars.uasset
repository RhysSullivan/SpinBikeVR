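; BP_Handlebars is a grabbable VR handlebar that turns its mesh as the holding motion controller moves.
; Grab stores the controller and its relative location, and Release clears the controller.
; While held, Tick adds the negated sum of the controller's X, Y and Z movement as yaw.
; Rotation applies only within the symmetric maximum steering limit, and the stored location updates only when it does.
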(event EventBeginPlay)

(event Collision|EventActorBeginOverlap
  (params (OtherActor :type Actor%20Object%20Reference)))

(event EventTick
  (params (DeltaSeconds :type Float%20%28single-precision%29))
  (bind _grabbedmotioncontroller (Variables|Default|GetGrabbedMotionController)
    (:then
      (if (and (<= (+ (* (+ (+ (.x (- (Variables|/Script/Engine.SceneComponent|GetRelativeLocation _grabbedmotioncontroller) (Variables|Default|GetMotionControllerOldRelativeTransform))) (.y (- (Variables|/Script/Engine.SceneComponent|GetRelativeLocation _grabbedmotioncontroller) (Variables|Default|GetMotionControllerOldRelativeTransform)))) (.z (- (Variables|/Script/Engine.SceneComponent|GetRelativeLocation _grabbedmotioncontroller) (Variables|Default|GetMotionControllerOldRelativeTransform)))) -1.0) (.yaw (Variables|/Script/Engine.SceneComponent|GetRelativeRotation (Variables|Default|GetStaticMesh)))) (Variables|Default|GetMaxSteeringWheelRotation)) (>= (+ (* (+ (+ (.x (- (Variables|/Script/Engine.SceneComponent|GetRelativeLocation _grabbedmotioncontroller) (Variables|Default|GetMotionControllerOldRelativeTransform))) (.y (- (Variables|/Script/Engine.SceneComponent|GetRelativeLocation _grabbedmotioncontroller) (Variables|Default|GetMotionControllerOldRelativeTransform)))) (.z (- (Variables|/Script/Engine.SceneComponent|GetRelativeLocation _grabbedmotioncontroller) (Variables|Default|GetMotionControllerOldRelativeTransform)))) -1.0) (.yaw (Variables|/Script/Engine.SceneComponent|GetRelativeRotation (Variables|Default|GetStaticMesh)))) (* (Variables|Default|GetMaxSteeringWheelRotation) -1.0)))
        (Transformation|AddRelativeRotation (Variables|Default|GetStaticMesh) (Math|Rotator|MakeRotator 0.0 0.0 (* (+ (+ (.x (- (Variables|/Script/Engine.SceneComponent|GetRelativeLocation _grabbedmotioncontroller) (Variables|Default|GetMotionControllerOldRelativeTransform))) (.y (- (Variables|/Script/Engine.SceneComponent|GetRelativeLocation _grabbedmotioncontroller) (Variables|Default|GetMotionControllerOldRelativeTransform)))) (.z (- (Variables|/Script/Engine.SceneComponent|GetRelativeLocation _grabbedmotioncontroller) (Variables|Default|GetMotionControllerOldRelativeTransform)))) -1.0)) false false)
        (Variables|Default|SetMotionControllerOldRelativeTransform (Variables|/Script/Engine.SceneComponent|GetRelativeLocation (Variables|Default|GetGrabbedMotionController)))))
    (:else)))

(fn ConstructionScript)

(fn Grab
  (params (WhichHand :type EControllerHand%20Enum :default "Left") (GrabbingActor :type Actor%20Object%20Reference) (MotionControllerComponent :type Scene%20Component%20Object%20Reference) (Socket%20To%20Attach%20To :type Name :default "None"))
  (Variables|Default|SetGrabbedMotionController MotionControllerComponent)
  (Variables|Default|SetMotionControllerOldRelativeTransform (Variables|/Script/Engine.SceneComponent|GetRelativeLocation (Variables|Default|GetGrabbedMotionController)))
  (return true self))

(fn Release
  (Variables|Default|SetGrabbedMotionController 0)
  (return true))