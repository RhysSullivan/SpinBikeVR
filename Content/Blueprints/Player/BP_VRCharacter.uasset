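; VR player character that provides motion-controller hands, turning and a blackout effect.
; On BeginPlay it resets the headset pose, sets eye-level tracking, then spawns left and right hand actors attached to their motion controllers.
; Input is forwarded to the hands for grab, use, trigger, pause and laser pointer debug, while turn presses rotate VROrigin in fixed steps.
; Blackout drives a plane material's opacity through a timeline.
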(event Custom|Blackout
  (bind _newtrack_0 (Timeline|Timeline_0 PlayFromStart)
    (:Update
      (Rendering|Material|SetScalarParameterValueonMaterials (Variables|Default|GetPlane) "Opacity" _newtrack_0))))

(event EventBeginPlay
  (Utilities|FlowControl|Sequence
    (:then_0
      (Class|HeadMountedDisplayFunctionLibrary|ResetOrientationandPosition 0.0 "OrientationAndPosition")
      (Class|HeadMountedDisplayFunctionLibrary|SetTrackingOrigin "Eye"))
    (:then_1
      (Utilities|FlowControl|Sequence
        (:then_0
          (bind _returnvalue (Game|SpawnActorfromClass "/Game/Blueprints/Player/BP_LeftHand.BP_LeftHand_C" (Math|Transform|MakeTransform "0, 0, 0" "0, 0, 0" "1,1,1") "Undefined" 0 0))
          (bind _output_get (Variables|Default|SetBP%20Left%20Hand _returnvalue))
          (Transformation|AttachComponentToComponent _output_get (Variables|Default|GetLeftMotionController) "None" "SnapToTarget" "SnapToTarget" "KeepWorld" false)
          (Variables|/Game/Blueprints/Player/BP_Hand.BP_Hand_C|SetMotionControllerComponent (Variables|Default|GetBP%20Left%20Hand) (Variables|Default|GetLeftMotionController)))
        (:then_1
          (bind _returnvalue_2 (Game|SpawnActorfromClass "/Game/Blueprints/Player/BP_RightHand.BP_RightHand_C" (Math|Transform|MakeTransform "0, 0, 0" "0, 0, 0" "1,1,1") "Undefined" 0 0))
          (bind _output_get_2 (Variables|Default|SetBP%20Right%20Hand _returnvalue_2))
          (Transformation|AttachComponentToComponent _output_get_2 (Variables|Default|GetRightMotionController) "None" "SnapToTarget" "SnapToTarget" "KeepWorld" false)
          (Variables|/Game/Blueprints/Player/BP_Hand.BP_Hand_C|SetMotionControllerComponent (Variables|Default|GetBP%20Right%20Hand) (Variables|Default|GetRightMotionController)))))))

(event Input|ActionEvents|InputActionTurnLeft
  (params (Key :type Key%20Structure :default "None"))
  (:Pressed
    (Transformation|AddWorldRotation (Variables|Default|GetVROrigin) (Math|Rotator|MakeRotator 0.0 0.0 (* (Variables|Default|GetRotationRate) -1.0)) false false)))

(event Input|ActionEvents|InputActionGrabRight
  (params (Key :type Key%20Structure :default "None"))
  (bind _bp_right_hand (Variables|Default|GetBP%20Right%20Hand))
  (:Pressed
    (Default|SendGrab _bp_right_hand))
  (:Released
    (Default|SendRelease _bp_right_hand)))

(event Input|ActionEvents|InputActionGrabLeft
  (params (Key :type Key%20Structure :default "None"))
  (bind _bp_left_hand (Variables|Default|GetBP%20Left%20Hand))
  (:Pressed
    (Default|SendGrab _bp_left_hand))
  (:Released
    (Default|SendRelease _bp_left_hand)))

(event Input|ActionEvents|InputActionUseRight
  (params (Key :type Key%20Structure :default "None"))
  (:Pressed
    (Default|Use (Variables|Default|GetBP%20Right%20Hand))))

(event Input|ActionEvents|InputActionPause
  (params (Key :type Key%20Structure :default "None"))
  (:Pressed
    (Default|Pause (Variables|Default|GetBP%20Left%20Hand))))

(event Input|ActionEvents|InputActionTurnRight
  (params (Key :type Key%20Structure :default "None"))
  (:Pressed
    (Transformation|AddWorldRotation (Variables|Default|GetVROrigin) (Math|Rotator|MakeRotator 0.0 0.0 (Variables|Default|GetRotationRate)) false false)))

(event Input|ActionEvents|InputActionToggleLaserPointer
  (params (Key :type Key%20Structure :default "None"))
  (bind _bp_right_hand (Variables|Default|GetBP%20Right%20Hand))
  (bind _widgetinteraction (Variables|/Game/Blueprints/Player/BP_RightHand.BP_RightHand_C|GetWidgetInteraction _bp_right_hand))
  (:Pressed
    (Variables|/Script/UMG.WidgetInteractionComponent|SetbShowDebug _widgetinteraction (not (Variables|/Script/UMG.WidgetInteractionComponent|GetbShowDebug _widgetinteraction)))))

(event Input|ActionEvents|InputActionMotionControllerTrigger
  (params (Key :type Key%20Structure :default "None"))
  (:Pressed
    (Default|TriggerPressed (Variables|Default|GetBP%20Right%20Hand))))

(fn ConstructionScript)