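; Right-hand player actor that handles pointing, interaction and dog commands during Agility mode.
; Each tick it traces forward to focus actors, range-limiting grabbables, and in Agility lays a movement icon on the traced surface.
; Use clicks through widget interaction, places or moves the dog's target actor at the icon in Agility, then activates the focused actor.
; In Agility, the trigger whistles and makes the dog jump.
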(event Custom|Activate
  (bind _lasthitactor (Variables|Default|GetLastHitActor)
    (:then
      (Class|BPWorldTraceInterface|Activate(Message) _lasthitactor self))
    (:else)))

(event Custom|Use
  (bind _widgetinteraction (Variables|Default|GetWidgetInteraction))
  (Class|WidgetInteractionComponent|PressPointerKey _widgetinteraction "LeftMouseButton")
  (Utilities|FlowControl|Delay 0.2)
  (Class|WidgetInteractionComponent|ReleasePointerKey _widgetinteraction "LeftMouseButton")
  (CallFunction|DoSpecialTaskBasedonDogState)
  (CallFunction|Activate))

(event Custom|SetMovementIconComponentLocation
  (bind _returnvalue (Transformation|GetActorLocation))
  (bind _movementicon (Variables|Default|GetMovementIcon))
  (bind (_outhit _returnvalue_2) (Collision|LineTraceByChannel _returnvalue (+ _returnvalue (* (Transformation|GetActorForwardVector) 1e+04)) "TraceTypeQuery1" false 0 "None"))
  (if _returnvalue_2
    (Transformation|SetWorldTransform (Variables|Default|GetMovementIcon) (Math|Transform|MakeTransform (.location _outhit) (Math|Rotator|MakeRotator (.roll (Math|Rotator|MakeRotfromXZ (Math|Vector|GetForwardVector _movementicon) (.impactnormal _outhit))) (.pitch (Class|KismetMathLibrary|MakeRotfromYZ (Math|Vector|GetRightVector _movementicon) (.impactnormal _outhit))) (.yaw (Math|Rotator|MakeRotfromXZ (Math|Vector|GetForwardVector _movementicon) (.impactnormal _outhit)))) "1,1,1") false false)))

(event Custom|TriggerPressed
  (bind _returnvalue (Game|Player|GetPlayerPawn 0))
  (bind _dog (Variables|Default|GetDog)
    (:then
      (bind _asbp_aicontroller_dog (Utilities|Casting|CastToBP_AIControllerDog (Pawn|GetController _dog)))
      (switch Utilities|FlowControl|Switch|SwitchonE_DogTask (Variables|/Game/Blueprints/AI/BP_AIControllerDog.BP_AIControllerDog_C|GetDogState _asbp_aicontroller_dog)
        (:NewEnumerator3
          (Audio|PlaySoundatLocation "/Game/Sound/Premade/Soundly/Human__Whistle_Fingers__Attention_SND23752.Human__Whistle_Fingers__Attention_SND23752" (Transformation|GetActorLocation _returnvalue) (Transformation|GetActorRotation _returnvalue) 1.0 1.0 0.0 "/Game/Sound/BarkAttinuation.BarkAttinuation" 0 0)
          (Utilities|FlowControl|Delay 0.2)
          (Character|Jump (Variables|Default|GetDog)))))
    (:else)))

(event EventBeginPlay)

(event Collision|EventActorBeginOverlap
  (params (OtherActor :type Actor%20Object%20Reference)))

(event EventTick
  (params (DeltaSeconds :type Float%20%28single-precision%29))
  (CallFunction|DoInteractTrace)
  (bind _dog (Variables|Default|GetDog)
    (:then
      (bind _asbp_aicontroller_dog (Utilities|Casting|CastToBP_AIControllerDog (Pawn|GetController _dog)))
      (switch Utilities|FlowControl|Switch|SwitchonE_DogTask (Variables|/Game/Blueprints/AI/BP_AIControllerDog.BP_AIControllerDog_C|GetDogState _asbp_aicontroller_dog)
        (:NewEnumerator3
          (CallFunction|SetMovementIconComponentLocation))))
    (:else)))

(fn ConstructionScript
  (|CallParentFunction))

(fn DoInteractTrace
  (bind _returnvalue (Transformation|GetActorLocation))
  (bind _outhit (Collision|LineTraceByChannel _returnvalue (+ _returnvalue (* (Transformation|GetActorForwardVector) 1e+04)) "TraceTypeQuery3" false 0 "None"))
  (if (.bblockinghit _outhit)
    (if (not (== (.hitactor _outhit) (Variables|Default|GetLastHitActor)))
      (bind _lasthitactor (Variables|Default|GetLastHitActor)
        (:then
          (Class|BPWorldTraceInterface|Unfocused(Message) _lasthitactor))
        (:else
          _))
      (Utilities|Casting|CastToBP_Grabbable (.hitactor _outhit)
        (:then
          (if (< (.distance _outhit) (Variables|Default|GetGrabbableDistance))
            (bind _output_get (Variables|Default|SetLastHitActor (.hitactor _outhit)))
            (Class|BPWorldTraceInterface|Focused(Message) _output_get)))
        (:CastFailed
          (bind _output_get_2 (Variables|Default|SetLastHitActor (.hitactor _outhit)))
          (Class|BPWorldTraceInterface|Focused(Message) _output_get_2))))
    (else
      (Variables|Default|SetLastHitActor 0))))

(fn DoSpecialTaskBasedonDogState
  (bind _dog (Variables|Default|GetDog)
    (:then
      (bind _asbp_aicontroller_dog (Utilities|Casting|CastToBP_AIControllerDog (Pawn|GetController _dog)))
      (switch Utilities|FlowControl|Switch|SwitchonE_DogTask (Variables|/Game/Blueprints/AI/BP_AIControllerDog.BP_AIControllerDog_C|GetDogState _asbp_aicontroller_dog)
        (:NewEnumerator3
          (Variables|Default|GetMovementIconActor
            (:then
              (Transformation|SetActorTransform (Variables|Default|GetMovementIconActor) (Transformation|GetWorldTransform (Variables|Default|GetMovementIcon)))
              (bind _output_get (Variables|/Game/Blueprints/AI/BP_AIControllerDog.BP_AIControllerDog_C|SetUserSetLocationActor _asbp_aicontroller_dog (Variables|Default|GetMovementIconActor)))
              (Rendering|SetActorHiddenInGame _output_get false))
            (:else
              (bind _returnvalue (Game|SpawnActorfromClass "/Game/Blueprints/ParkProps/AgilityCourse/BP_AgilityMovementLocation.BP_AgilityMovementLocation_C" (Transformation|GetWorldTransform (Variables|Default|GetMovementIcon)) "Undefined" 0 0))
              (bind _output_get_2 (Variables|Default|SetMovementIconActor _returnvalue))
              (Variables|/Game/Blueprints/AI/BP_AIControllerDog.BP_AIControllerDog_C|SetUserSetLocationActor _asbp_aicontroller_dog _output_get_2))))))
    (:else)))