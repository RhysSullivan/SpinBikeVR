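; BP_BikeGamemode is the game mode for a bike game, built around a two-player session.
; It pauses the game on BeginPlay and, on the authority, unpauses it in PostLogin once the player count equals two.
; Its GetDefaultPawnClassForController override returns BP_Spectator when the player count is exactly two, otherwise deferring to the parent's default pawn class.
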(event EventBeginPlay
  (Game|SetGamePaused true))

(event EventPostLogin
  (params (NewPlayer :type Player%20Controller%20Object%20Reference))
  (if (Ability|HasAuthority)
    (bind _returnvalue (Class|GameModeBase|GetNumPlayers))
    (if (== _returnvalue 2)
      (Game|SetGamePaused false))))

(fn ConstructionScript)

(fn GetDefaultPawnClassforController
  (params (InController :type Controller%20Object%20Reference))
  (bind _returnvalue (|CallParentFunction InController))
  (bind _returnvalue_2 (Class|GameModeBase|GetNumPlayers))
  (if (== _returnvalue_2 2)
    (return "/Game/Blueprints/BP_Spectator.BP_Spectator_C")
    (else
      (return _returnvalue))))