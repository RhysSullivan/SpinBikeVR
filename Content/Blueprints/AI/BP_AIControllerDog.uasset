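; AI controller for the VR game's dog companion, driving movement for its Fetch and Agility states.
; Tick calls hand-written per-state events that issue AIMoveTo, with no Behavior Tree asset.
; Fetch chases the loose ball, or brings it before the player's camera when it is attached outside the hand.
; Agility heads to a user-set marker, otherwise optionally straight ahead, widening acceptance radius while airborne.
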(event Custom|Fetch%20Behavior%20Tree
  (if (CallFunction|CanChaseBall)
    (if (not (== (Actor|GetAttachParentActor (Variables|Default|GetBall)) "/Game/Blueprints/Player/BP_Hand.BP_Hand"))
      (bind _asbp_vrcharacter (Utilities|Casting|CastToBP_VRCharacter (Game|Player|GetPlayerPawn 0)))
      (AI|AIMoveTo (Pawn|GetControlledPawn) (.ProjectedLocation (AI|Navigation|ProjectPointtoNavigation (+ (Transformation|GetWorldLocation (Variables|/Game/Blueprints/Player/BP_VRCharacter.BP_VRCharacter_C|GetCamera _asbp_vrcharacter)) (* (Math|Vector|GetForwardVector (Variables|/Game/Blueprints/Player/BP_VRCharacter.BP_VRCharacter_C|GetCamera _asbp_vrcharacter)) 1e+02)) 0 0 "500.000000,500.000000,500.000000")) 0 1e+02 false
        (:OnSuccess
          (Transformation|SetActorRotation (Math|Rotator|MakeRotator (.roll (Math|Rotator|FindLookatRotation (Transformation|GetActorLocation (Pawn|GetControlledPawn)) (Transformation|GetWorldLocation (Variables|/Game/Blueprints/Player/BP_VRCharacter.BP_VRCharacter_C|GetCamera _asbp_vrcharacter)))) (.pitch (Math|Rotator|FindLookatRotation (Transformation|GetActorLocation (Pawn|GetControlledPawn)) (Transformation|GetWorldLocation (Variables|/Game/Blueprints/Player/BP_VRCharacter.BP_VRCharacter_C|GetCamera _asbp_vrcharacter)))) (.yaw (Math|Rotator|FindLookatRotation (Transformation|GetActorLocation (Pawn|GetControlledPawn)) (Transformation|GetWorldLocation (Variables|/Game/Blueprints/Player/BP_VRCharacter.BP_VRCharacter_C|GetCamera _asbp_vrcharacter)))))))))
    (else
      (Variables|Default|SetDogChaseState "NewEnumerator0")
      (AI|AIMoveTo (Pawn|GetControlledPawn) (.ProjectedLocation (AI|Navigation|ProjectPointtoNavigation (Transformation|GetActorLocation (Variables|Default|GetBall)) 0 0 "1000.000000,1000.000000,10000.000000")) 0 2e+01 false))))

(event Custom|AgilityBehaviorTree
  (bind _dog (Variables|Default|GetDog))
  (bind _mesh (Variables|/Script/Engine.Character|GetMesh _dog))
  (bind _returnvalue (Math|Vector|GetRightVector _mesh))
  (if (AI|Components|NavMovement|IsFalling (Variables|/Script/Engine.Character|GetCharacterMovement (Variables|Default|GetDog)))
    (Variables|Default|SetAgilityAcceptanceRadius 2.5e+02)
    (else
      (Variables|Default|SetAgilityAcceptanceRadius 2e+01)))
  (Variables|Default|GetUserSetLocationActor
    (:then
      (AI|AIMoveTo (Pawn|GetControlledPawn) "0, 0, 0" (Variables|Default|GetUserSetLocationActor) (Variables|Default|GetAgilityAcceptanceRadius) false
        (:OnSuccess
          (bind _usersetlocationactor (Variables|Default|GetUserSetLocationActor)
            (:then
              (Rendering|SetActorHiddenInGame _usersetlocationactor true)
              (Variables|Default|SetUserSetLocationActor 0))
            (:else)))))
    (:else
      (if (Variables|Default|GetMoveToForwardVector)
        (AI|AIMoveTo 0 (+ (* (Math|Vector|MakeVector (.x _returnvalue) (.y _returnvalue) 0.0) 1e+03) (Transformation|GetWorldLocation _mesh)) 0 5.0 false)))))

(event EventBeginPlay
  (bind _asbp_aidog (Utilities|Casting|CastToBP_AIDog (Pawn|GetControlledPawn)))
  (Variables|Default|SetDog _asbp_aidog))

(event EventTick
  (params (DeltaSeconds :type Float%20%28single-precision%29))
  (switch Utilities|FlowControl|Switch|SwitchonE_DogTask (Variables|Default|GetDogState)
    (:NewEnumerator1
      (CallFunction|FetchBehaviorTree))
    (:NewEnumerator3
      (CallFunction|AgilityBehaviorTree))))

(fn ConstructionScript)

(fn CanChaseBall
  (bind _asbp_aidog (Utilities|Casting|CastToBP_AIDog (Pawn|GetControlledPawn)))
  (bind _ball (Variables|/Game/Blueprints/AI/BP_AIDog.BP_AIDog_C|GetBall _asbp_aidog)
    (:then
      (bind _output_get (Variables|Default|SetBall _ball))
      (return (Utilities|IsValid (Actor|GetAttachParentActor _output_get))))
    (:else
      (return false))))

(fn SetDogState
  (params (DogState :type E_DogTask%20Enum :default "NewEnumerator0"))
  (switch Utilities|FlowControl|Switch|SwitchonE_DogTask (Variables|Default|GetDogState)
    (:NewEnumerator0
      _)
    (:NewEnumerator1
      _)
    (:NewEnumerator2
      _)
    (:NewEnumerator3
      (bind _usersetlocationactor (Variables|Default|GetUserSetLocationActor)
        (:then
          (Actor|DestroyActor _usersetlocationactor))
        (:else
          _))))
  (bind _output_get (Variables|Default|SetDogState DogState))
  (switch Utilities|FlowControl|Switch|SwitchonE_DogTask _output_get
    (:NewEnumerator0
      _)
    (:NewEnumerator1
      _)
    (:NewEnumerator2
      _)
    (:NewEnumerator3
      _))
  (Components|Animation|SetAnimationMode (Variables|/Script/Engine.Character|GetMesh (Variables|Default|GetDog)) "AnimationBlueprint")
  (Components|SkeletalMesh|SetAnimInstanceClass (Variables|/Script/Engine.Character|GetMesh (Variables|Default|GetDog)) "/Game/Art/AnimationBlueprint/ABP_Dog.ABP_Dog_C"))