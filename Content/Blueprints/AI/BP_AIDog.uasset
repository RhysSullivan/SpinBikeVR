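; AI dog character for a VR game that plays fetch with grabbable objects when its controller is in the Fetch state.
; Tick aligns the body to the ground with a downward trace and times how long the player's hands have been empty.
; That timer gates two overlap triggers: one jumps at free objects, the other attaches Ball to the jaw socket.
; Also handles random sounds, a black-coat variant and sprint/rest speed helpers.
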(event OnComponentBeginOverlap(Box)
  (params (OverlappedComponent :type Primitive%20Component%20Object%20Reference) (OtherActor :type Actor%20Object%20Reference) (OtherComp :type Primitive%20Component%20Object%20Reference) (OtherBodyIndex :type Integer) (bFromSweep :type Boolean) (SweepResult :type Hit%20Result%20Structure%20%28by%20ref%29))
  (bind _asbp_aicontroller_dog (Utilities|Casting|CastToBP_AIControllerDog (Pawn|GetController)))
  (switch Utilities|FlowControl|Switch|SwitchonE_DogTask (Variables|/Game/Blueprints/AI/BP_AIControllerDog.BP_AIControllerDog_C|GetDogState _asbp_aicontroller_dog)
    (:NewEnumerator1
      (if (> (Variables|Default|GetTimeSinceThrow) (Variables|Default|GetTimeToWaitBeforePickingUp))
        (if (not (Utilities|IsValid (Actor|GetAttachParentActor OtherActor)))
          (bind _asbp_grabbable (Utilities|Casting|CastToBP_Grabbable OtherActor))
          (Default|TogglePhysics _asbp_grabbable false)
          (bind _ball (Variables|Default|GetBall)
            (:then
              (Transformation|AttachComponentToComponent _ball (Variables|Character|GetMesh) "jawSocket" "SnapToTarget" "SnapToTarget" "KeepWorld" true)
              (Default|CallDogGotGoal))
            (:else)))))))

(event OnComponentBeginOverlap(Jump)
  (params (OverlappedComponent :type Primitive%20Component%20Object%20Reference) (OtherActor :type Actor%20Object%20Reference) (OtherComp :type Primitive%20Component%20Object%20Reference) (OtherBodyIndex :type Integer) (bFromSweep :type Boolean) (SweepResult :type Hit%20Result%20Structure%20%28by%20ref%29))
  (bind _asbp_aicontroller_dog (Utilities|Casting|CastToBP_AIControllerDog (Pawn|GetController)))
  (switch Utilities|FlowControl|Switch|SwitchonE_DogTask (Variables|/Game/Blueprints/AI/BP_AIControllerDog.BP_AIControllerDog_C|GetDogState _asbp_aicontroller_dog)
    (:NewEnumerator1
      (if (> (Variables|Default|GetTimeSinceThrow) (Variables|Default|GetTimeToWaitBeforeJumping))
        (if (not (Utilities|IsValid (Actor|GetAttachParentActor OtherActor)))
          (Utilities|Casting|CastToBP_Grabbable OtherActor)
          (Character|Jump))))))

(event Custom|DoDogSound
  (Utilities|FlowControl|Delay (Math|Random|RandomFloatinRange 5.0 1e+01))
  (Audio|SpawnSoundatLocation (Utilities|Array|Get(acopy) (Variables|Default|GetSoundArray) (Math|Random|RandomIntegerinRange 0 2)) (Transformation|GetActorLocation) (Transformation|GetActorRotation) 1.0 1.0 0.0 "/Game/Sound/BarkAttinuation.BarkAttinuation" 0)
  (CallFunction|DoDogSound))

(event Custom|MatchSlope
  (params (DeltaTime :type Float%20%28single-precision%29))
  (bind _returnvalue (Transformation|GetActorLocation))
  (bind _outhit (Collision|LineTraceByChannel _returnvalue (+ _returnvalue (* (Transformation|GetActorUpVector) (* (Variables|Default|GetGapDistance) -1.0))) "TraceTypeQuery1" false 0 "None"))
  (if (.bblockinghit _outhit)
    (Transformation|SetActorRotation (Class|KismetMathLibrary|RInterptoConstant (Transformation|GetActorRotation) (Math|Rotator|MakeRotator (.roll (Math|Rotator|MakeRotator (.roll (Math|Rotator|MakeRotfromXZ (Transformation|GetActorForwardVector) (.impactnormal _outhit))) (.pitch (Class|KismetMathLibrary|MakeRotfromYZ (Transformation|GetActorRightVector) (.impactnormal _outhit))) (.yaw (Math|Rotator|MakeRotfromXZ (Transformation|GetActorForwardVector) (.impactnormal _outhit))))) (.pitch (Math|Rotator|MakeRotator (.roll (Math|Rotator|MakeRotfromXZ (Transformation|GetActorForwardVector) (.impactnormal _outhit))) (.pitch (Class|KismetMathLibrary|MakeRotfromYZ (Transformation|GetActorRightVector) (.impactnormal _outhit))) (.yaw (Math|Rotator|MakeRotfromXZ (Transformation|GetActorForwardVector) (.impactnormal _outhit))))) (.yaw (Transformation|GetActorRotation))) DeltaTime 5e+01))))

(event Custom|SetWalkSpeedBasedOnRecovery
  (if (> (Variables|Default|GetTimeSpentRecovering) (Variables|Default|GetRecoveryTime))
    (if (> (Variables|Default|GetTimeSpentSprintingTime) (Variables|Default|GetAllocatedSprintingTime))
      (Variables|/Script/Engine.CharacterMovementComponent|SetMaxWalkSpeed (Variables|Character|GetCharacterMovement) (Variables|Default|GetRestingSpeed))
      (else
        (Variables|/Script/Engine.CharacterMovementComponent|SetMaxWalkSpeed (Variables|Character|GetCharacterMovement) (Variables|Default|GetSprintingSpeed))
        (Variables|Default|SetTimeSpentSprintingTime 0.0)))
    (else
      (Variables|/Script/Engine.CharacterMovementComponent|SetMaxWalkSpeed (Variables|Character|GetCharacterMovement) (Variables|Default|GetRestingSpeed)))))

(event EventTick
  (params (DeltaSeconds :type Float%20%28single-precision%29))
  (CallFunction|MatchSlope DeltaSeconds)
  (bind _asbp_aicontroller_dog (Utilities|Casting|CastToBP_AIControllerDog (Pawn|GetController)))
  (switch Utilities|FlowControl|Switch|SwitchonE_DogTask (Variables|/Game/Blueprints/AI/BP_AIControllerDog.BP_AIControllerDog_C|GetDogState _asbp_aicontroller_dog)
    (:NewEnumerator1
      (bind _asbp_vrcharacter (Utilities|Casting|CastToBP_VRCharacter (Game|Player|GetPlayerPawn 0)))
      (bind _returnvalue (CallFunction|FindAttachedActoronEitherHand (Variables|/Game/Blueprints/Player/BP_VRCharacter.BP_VRCharacter_C|GetBP%20Right%20Hand _asbp_vrcharacter) (Variables|/Game/Blueprints/Player/BP_VRCharacter.BP_VRCharacter_C|GetBP%20Left%20Hand _asbp_vrcharacter)))
      (Utilities|IsValid _returnvalue
        (:Is%20Valid
          (Variables|Default|SetPlayerHasObject true)
          (Variables|Default|SetTimeSinceThrow 0.0))
        (:Is%20Not%20Valid
          (Variables|Default|SetTimeSinceThrow (+ (Variables|Default|GetTimeSinceThrow) DeltaSeconds)))))))

(event EventBeginPlay
  (Variables|Default|SetGapDistance (- (.z (Transformation|GetActorLocation)) (- (.z (Transformation|GetWorldLocation (Variables|Default|GetTraceEnd))) 3e+01)))
  (CallFunction|DoDogSound)
  (bind _asbp_game_instance (Utilities|Casting|CastToBP_GameInstance (Game|GetGameInstance)))
  (if (Variables|/Game/Blueprints/General/BP_GameInstance.BP_GameInstance_C|GetChoseChoiceCorgiBlack _asbp_game_instance)
    (Rendering|Material|SetMaterial (Variables|Character|GetMesh) 1 "/Game/Art/Materials/M_DogMaterialBlack.M_DogMaterialBlack")
    (Rendering|Material|SetMaterial (Variables|Character|GetMesh) 2 "/Game/Art/Materials/M_DogMaterialBlack.M_DogMaterialBlack")
    (Variables|Default|SetNameOfDog "Midnight")))

(fn ConstructionScript)

(fn FindAttachedActoronEitherHand
  (params (LeftHand :type Actor%20Object%20Reference) (RightHand :type Actor%20Object%20Reference))
  (bind _outactors (Actor|GetAttachedActors RightHand))
  (bind _outactors_2 (Actor|GetAttachedActors LeftHand))
  (if (Utilities|Array|IsValidIndex _outactors_2)
    (return (Utilities|Array|Get(acopy) _outactors_2))
    (elif (Utilities|Array|IsValidIndex _outactors)
      (return (Utilities|Array|Get(acopy) _outactors)))))

(fn FindTimeSpentinState
  (params (Deltatime :type Float%20%28single-precision%29))
  (if (> (Math|Vector|VectorLength (Pawn|Components|CharacterMovement|GetLastUpdateVelocity (Variables|Character|GetCharacterMovement))) (+ (Variables|Default|GetRestingSpeed) 2e+01))
    (Variables|Default|SetTimeSpentSprintingTime (+ (Variables|Default|GetTimeSpentSprintingTime) Deltatime))
    (else
      (Variables|Default|SetTimeSpentRecovering (+ (Variables|Default|GetTimeSpentRecovering) Deltatime)))))