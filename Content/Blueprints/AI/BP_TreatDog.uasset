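; BP_TreatDog is a dog actor that catches grabbable objects, presumably treats, in its mouth.
; On BeginPlay it swaps two skeletal mesh material slots to black if the game instance records the black corgi choice.
; When its lower jaw collision hits a BP_Grabbable, it turns off that object's physics and collision, snaps it to the jaw socket and stores it as TreatInMouth.
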(event OnComponentHit(LowJawCollision)
  (params (HitComponent :type Primitive%20Component%20Object%20Reference) (OtherActor :type Actor%20Object%20Reference) (OtherComp :type Primitive%20Component%20Object%20Reference) (NormalImpulse :type Vector :default "0, 0, 0") (Hit :type Hit%20Result%20Structure%20%28by%20ref%29))
  (bind _asbp_grabbable (Utilities|Casting|CastToBP_Grabbable OtherActor))
  (Default|TogglePhysics _asbp_grabbable false)
  (Transformation|AttachComponentToComponent _asbp_grabbable (Variables|Default|GetSkeletalMesh) "jawSocket" "SnapToTarget" "SnapToTarget" "KeepWorld" true)
  (Variables|Default|SetTreatInMouth _asbp_grabbable)
  (Collision|SetActorEnableCollision _asbp_grabbable false))

(event Collision|EventActorBeginOverlap
  (params (OtherActor :type Actor%20Object%20Reference)))

(event EventTick
  (params (DeltaSeconds :type Float%20%28single-precision%29)))

(event EventBeginPlay
  (bind _asbp_game_instance (Utilities|Casting|CastToBP_GameInstance (Game|GetGameInstance)))
  (if (Variables|/Game/Blueprints/General/BP_GameInstance.BP_GameInstance_C|GetChoseChoiceCorgiBlack _asbp_game_instance)
    (Rendering|Material|SetMaterial (Variables|Default|GetSkeletalMesh) 1 "/Game/Art/Materials/M_DogMaterialBlack.M_DogMaterialBlack")
    (Rendering|Material|SetMaterial (Variables|Default|GetSkeletalMesh) 2 "/Game/Art/Materials/M_DogMaterialBlack.M_DogMaterialBlack")))

(fn ConstructionScript)