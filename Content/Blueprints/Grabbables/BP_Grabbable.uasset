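; BP_Grabbable is a physics prop that hands or other actors can grab, activate and release.
; Grab and Activate both call Attach, which first frees it from any current parent, via SendRelease for a BP_Hand or ForceDrop otherwise, then disables physics and snaps it to the new actor.
; Release and ForceDrop re-enable mesh physics and detach it in place, keeping its world transform.
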(event Custom|Force%20Drop
  (CallFunction|TogglePhysics true)
  (Transformation|DetachFromActor "KeepWorld" "KeepWorld" "KeepWorld"))

(event Custom|Attach
  (params (Target :type Actor%20Object%20Reference))
  (Utilities|IsValid (Actor|GetAttachParentActor)
    (:Is%20Valid
      (bind _asbp_hand (Utilities|Casting|CastToBP_Hand (Actor|GetAttachParentActor))
        (:then
          (Default|SendRelease _asbp_hand))
        (:CastFailed
          (CallFunction|ForceDrop))))
    (:Is%20Not%20Valid
      _))
  (CallFunction|TogglePhysics false)
  (Transformation|AttachActorToActor Target "None" "SnapToTarget" "SnapToTarget" "KeepWorld" true))

(event EventActivate
  (params (SendingActor :type Actor%20Object%20Reference))
  (CallFunction|Attach SendingActor))

(fn ConstructionScript)

(fn TogglePhysics
  (params (PhysicsOn? :type Boolean))
  (Physics|SetSimulatePhysics (Variables|Default|GetStaticMesh) PhysicsOn?))

(fn Grab
  (params (WhichHand :type EControllerHand%20Enum :default "Left") (GrabbingActor :type Actor%20Object%20Reference) (MotionControllerComponent :type Scene%20Component%20Object%20Reference) (Socket%20To%20Attach%20To :type Name :default "None"))
  (CallFunction|Attach GrabbingActor)
  (return true self))

(fn Release
  (CallFunction|TogglePhysics true)
  (Transformation|DetachFromActor "KeepWorld" "KeepWorld" "KeepWorld")
  (return true))