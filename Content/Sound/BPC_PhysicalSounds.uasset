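; BPC_PhysicalSounds is an actor component that plays impact sounds when its owner's static meshes hit something.
; On BeginPlay it binds a hit handler to every StaticMeshComponent on the owner.
; Hits with a normal impulse above a minimum threshold play a configurable, attenuated sound at the hit location, with volume scaled linearly by impulse magnitude through a divisor.
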(event Custom|OnComponentHit_Event
  (params (HitComponent :type Primitive%20Component%20Object%20Reference) (OtherActor :type Actor%20Object%20Reference) (OtherComp :type Primitive%20Component%20Object%20Reference) (NormalImpulse :type Vector) (Hit :type Hit%20Result%20Structure%20%28by%20ref%29))
  (bind _returnvalue (Math|Vector|VectorLength NormalImpulse))
  (if (> _returnvalue (Variables|Default|GetSmallestImpluseToMakeSound))
    (Audio|PlaySoundatLocation (Variables|Default|GetSoundToPlay) (.location Hit) "0, 0, 0" (/ _returnvalue (Variables|Default|GetSoundDivision)) 1.0 0.0 (Variables|Default|GetAttinuation) 0 0)))

(event EventBeginPlay
  (for _array_element (Actor|GetComponentsByClass (Components|GetOwner) "/Script/Engine.StaticMeshComponent")
    (Collision|AssignOnComponentHit _array_element (delegate Custom|OnComponentHit_Event))))

(event EventTick
  (params (DeltaSeconds :type Float%20%28single-precision%29)))